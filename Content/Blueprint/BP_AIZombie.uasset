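; Zombie AI character that chases the first player and dies from accumulated damage.
; Tick reissues a simple move-to-actor toward the player every frame.
; AnyDamage subtracts from Health and prints a debug string while it survives.
; Once Health drops below zero, it disables movement, plays a death animation and collapse sound, then destroys itself after a short delay.
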(event EventTick
  (params (DeltaSeconds :type Float%20%28single-precision%29))
  (AI|Navigation|SimpleMovetoActor (Pawn|GetController) (Game|GetPlayerCharacter 0)))

(event Game|Damage|EventAnyDamage
  (params (Damage :type Float%20%28single-precision%29) (DamageType :type Damage%20Type%20Object%20Reference) (InstigatedBy :type Controller%20Object%20Reference) (DamageCauser :type Actor%20Object%20Reference))
  (Variables|Default|SetHealth (- (Variables|Default|GetHealth) Damage))
  (if (< (Variables|Default|GetHealth) 0.0)
    (Pawn|Components|CharacterMovement|SetMovementMode (Variables|Character|GetCharacterMovement) "MOVE_None" 0)
    (Components|Animation|PlayAnimation (Variables|Character|GetMesh) "/Game/AnimStarterPack/Prone_Death_1.Prone_Death_1" false)
    (Audio|PlaySoundatLocation "/Game/StarterContent/Audio/Collapse01.Collapse01" (Transformation|GetActorLocation) "0, 0, 0" 0.2 1.0 0.0 0 0 0 0)
    (Utilities|FlowControl|Delay 2.0)
    (Actor|DestroyActor)
    (else
      (Development|PrintString "DAMAGE"))))

(fn ConstructionScript)